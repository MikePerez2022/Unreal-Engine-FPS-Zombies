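; BP_MikeGM, apparently a game mode by its name, handles adding local players who each control a BP_Mike pawn.
; AddLocalPlayer waits briefly, creates a player at the running PlayerIndex, then possesses that player's pawn if it is a BP_Mike.
; It then calls the pawn's OnSpawn, stores the index on it and increments PlayerIndex and PlayerCount.
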(event `AddLocalPlayer`
  (bind _playerindex (`self.PlayerIndex`))
  (`KismetSystemLibrary.Delay` 0.2)
  (`GameplayStatics.CreatePlayer` _playerindex)
  (bind _asbp_mike (cast `/Game/Mike/BP_Mike` (`GameplayStatics.GetPlayerPawn` _playerindex)))
  (`Controller.Possess` (`GameplayStatics.GetPlayerController` (`self.PlayerIndex`)) _asbp_mike)
  (`/Game/FirstPerson/Blueprints/BP_FirstPersonCharacter.OnSpawn` _asbp_mike)
  (set `/Game/FirstPerson/Blueprints/BP_FirstPersonCharacter.PlayerIndex` (`self.PlayerIndex`) _asbp_mike)
  (`/Engine/EditorBlueprintResources/StandardMacros.IncrementInt` (`self.PlayerIndex`)
    (:`  `
      (`/Engine/EditorBlueprintResources/StandardMacros.IncrementInt` (`self.PlayerCount`)))))

(fn `UserConstructionScript`)