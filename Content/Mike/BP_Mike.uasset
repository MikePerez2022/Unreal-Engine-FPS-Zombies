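; BP_Mike is a Blueprint that gives its owner passive health regeneration.
; While JustHit is false, Tick starts a Delay, so health rises by RegenRate in spaced pulses rather than every frame, capped at MaxHealth.
; JustHit is checked only before the Delay, so a pending pulse still lands if the flag changes; nothing in these graphs sets it.
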(event `self.ReceiveTick`
  (params (DeltaSeconds :type "Float (single-precision)"))
  (bind _maxhealth (`self.MaxHealth`))
  (if (not (`self.JustHit`))
    (`KismetSystemLibrary.Delay` 2.5)
    (bind _output_get (set `self.Health` (+ (`self.Health`) (`self.RegenRate`))))
    (if (>= _output_get _maxhealth)
      (set `self.Health` _maxhealth))))

(fn `UserConstructionScript`
  (`parent.UserConstructionScript`))