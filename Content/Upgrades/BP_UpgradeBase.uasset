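; Base upgrade pickup actor that shows a purchase prompt and charges the player money for an upgrade.
; Overlapping its Box with a first-person character creates a WBP_Upgrade widget for that player's controller, filled with the upgrade's Name and Cost, and leaving removes it.
; The Upgrade function deducts Cost from the player's Money when affordable and returns whether the purchase succeeded.
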(event `self.Box.OnComponentBeginOverlap`
  (params (OverlappedComponent :type "PrimitiveComponent Object Reference") (OtherActor :type "Actor Object Reference") (OtherComp :type "PrimitiveComponent Object Reference") (OtherBodyIndex :type Integer) (bFromSweep :type Boolean) (SweepResult :type "HitResult Structure (by ref)"))
  (bind _asbp_first_person_character (cast `/Game/FirstPerson/Blueprints/BP_FirstPersonCharacter` OtherActor))
  (bind _returnvalue (`|CreateWidget` "/Game/Upgrades/WBP_Upgrade.WBP_Upgrade_C" (`GameplayStatics.GetPlayerController` (`/Game/FirstPerson/Blueprints/BP_FirstPersonCharacter.PlayerIndex` _asbp_first_person_character))))
  (bind _output_get (set `self.Widget` _returnvalue))
  (set `/Game/Upgrades/WBP_Upgrade.CostIn` (`self.Cost`) _output_get)
  (set `/Game/Upgrades/WBP_Upgrade.NameIn` (`self.Name`) _output_get)
  (`UserWidget.AddToViewport` _output_get 0))

(event `self.Box.OnComponentEndOverlap`
  (params (OverlappedComponent :type "PrimitiveComponent Object Reference") (OtherActor :type "Actor Object Reference") (OtherComp :type "PrimitiveComponent Object Reference") (OtherBodyIndex :type Integer))
  (cast `/Game/FirstPerson/Blueprints/BP_FirstPersonCharacter` OtherActor)
  (`Widget.RemoveFromParent` (`self.Widget`)))

(fn `Upgrade`
  (params (Player :type "/Game/FirstPerson/Blueprints/BP_FirstPersonCharacter Object Reference"))
  (returns (Bought :type Boolean))
  (bind _cost (`self.Cost`))
  (bind _money (`/Game/FirstPerson/Blueprints/BP_FirstPersonCharacter.Money` Player))
  (if (>= _money _cost)
    (set `/Game/FirstPerson/Blueprints/BP_FirstPersonCharacter.Money` (- _money _cost) Player)
    (return true)
    (else
      (return false))))

(fn `UserConstructionScript`)