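; BP_ExtraHealth is an upgrade Blueprint that raises a player's maximum health.
; Its Upgrade override calls the parent implementation first and, only when that returns true, sets the Player's MaxHealth to a fixed value rather than adding to it.
; Current health is not changed here, and the event graph holds only disabled default events.
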(fn `Upgrade`
  (params (Player :type "/Game/FirstPerson/Blueprints/BP_FirstPersonCharacter Object Reference"))
  (bind _bought (`parent.Upgrade` Player))
  (if _bought
    (set `/Game/FirstPerson/Blueprints/BP_FirstPersonCharacter.MaxHealth` 200.0 Player)))

(fn `UserConstructionScript`
  (`parent.UserConstructionScript`))