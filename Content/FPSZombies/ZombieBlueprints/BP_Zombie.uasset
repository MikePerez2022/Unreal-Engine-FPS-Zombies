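; BP_Zombie is a zombie enemy that takes damage and dies as a ragdoll.
; AnyDamage subtracts damage from Health; below zero, the mesh switches to physics simulation with physics-only collision and the capsule's collision is disabled.
; It then casts player 0's character to BP_FirstPersonCharacter to increment the kill count and calls SetLifeSpan with zero, which schedules no destruction.
; No guard prevents further damage from repeating the death sequence.
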(event `self.ReceiveBeginPlay`)

(event `self.ReceiveAnyDamage`
  (params (Damage :type "Float (single-precision)") (DamageType :type "DamageType Object Reference") (InstigatedBy :type "Controller Object Reference") (DamageCauser :type "Actor Object Reference"))
  (bind _mesh (`self.Mesh`))
  (bind _output_get (set `self.Health` (- (`self.Health`) Damage)))
  (if (< _output_get 0.0)
    (`PrimitiveComponent.SetSimulatePhysics` _mesh true)
    (`PrimitiveComponent.SetCollisionEnabled` _mesh "PhysicsOnly")
    (`PrimitiveComponent.SetCollisionEnabled` (`self.CapsuleComponent`) "NoCollision")
    (bind _asbp_first_person_character (cast `/Game/FirstPerson/Blueprints/BP_FirstPersonCharacter` (`GameplayStatics.GetPlayerCharacter` 0)))
    (`/Game/FirstPerson/Blueprints/BP_FirstPersonCharacter.Increment Kill Count` _asbp_first_person_character)
    (`self.SetLifeSpan` 0.0)))

(fn `UserConstructionScript`)