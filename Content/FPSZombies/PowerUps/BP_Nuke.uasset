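; BP_Nuke is a zombie-mode power-up that wipes out all zombies when a first-person character overlaps it.
; On overlap it loops over local player indices, adding a fixed bonus scaled by each character's money multiplier to their Money.
; Every BP_Zombie is destroyed directly inside that same loop, so the search repeats per player.
; The pickup then destroys itself.
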(event `self.ReceiveBeginPlay`
  (`parent.ReceiveBeginPlay`))

(event `self.ReceiveActorBeginOverlap`
  (params (OtherActor :type "Actor Object Reference"))
  (if (`KismetMathLibrary.ClassIsChildOf` (`GameplayStatics.GetObjectClass` OtherActor) "/Game/FirstPerson/Blueprints/BP_FirstPersonCharacter.BP_FirstPersonCharacter_C")
    (for _index (range (+ (`GameplayStatics.GetNumLocalPlayerControllers`) 1))
      (bind _asbp_first_person_character (cast `/Game/FirstPerson/Blueprints/BP_FirstPersonCharacter` (`GameplayStatics.GetPlayerPawn` _index)))
      (set `/Game/FirstPerson/Blueprints/BP_FirstPersonCharacter.Money` (+ (`/Game/FirstPerson/Blueprints/BP_FirstPersonCharacter.Money` _asbp_first_person_character) (* (`/Game/FirstPerson/Blueprints/BP_FirstPersonCharacter.MoneyMult` _asbp_first_person_character) 400)) _asbp_first_person_character)
      (bind _outactors (`GameplayStatics.GetAllActorsOfClass` "/Game/FPSZombies/ZombieBlueprints/BP_Zombie.BP_Zombie_C"))
      (for _array_element _outactors
        (`self.K2_DestroyActor` _array_element)))
    (`self.K2_DestroyActor`)))

(fn `UserConstructionScript`
  (`parent.UserConstructionScript`))