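; BP_MaxAmmo is a power-up pickup in the FPS zombies game that refills the player's ammo.
; On overlap with the first player's pawn, it casts to BP_FirstPersonCharacter and sets CurrentAmmo to MaxAmmo.
; It then destroys itself, so each pickup works once.
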(event `self.ReceiveBeginPlay`
  (`parent.ReceiveBeginPlay`))

(event `self.ReceiveActorBeginOverlap`
  (params (OtherActor :type "Actor Object Reference"))
  (bind _returnvalue (`GameplayStatics.GetPlayerPawn` 0))
  (if (== OtherActor _returnvalue)
    (bind _asbp_first_person_character (cast `/Game/FirstPerson/Blueprints/BP_FirstPersonCharacter` _returnvalue))
    (set `/Game/FirstPerson/Blueprints/BP_FirstPersonCharacter.CurrentAmmo` (`/Game/FirstPerson/Blueprints/BP_FirstPersonCharacter.MaxAmmo` _asbp_first_person_character) _asbp_first_person_character)
    (`self.K2_DestroyActor`)))

(fn `UserConstructionScript`
  (`parent.UserConstructionScript`))