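; Double-points power-up pickup for the FPS zombies game, triggered when an actor of the first-person character class overlaps it.
; On overlap it loops over local player controller indices and calls DoublePointsActivated on each player's character, so the bonus is shared by all local players.
; The pickup then destroys itself, leaving the effect itself to the character Blueprint.
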(event `self.ReceiveBeginPlay`
  (`parent.ReceiveBeginPlay`))

(event `self.ReceiveActorBeginOverlap`
  (params (OtherActor :type "Actor Object Reference"))
  (if (`KismetMathLibrary.ClassIsChildOf` (`GameplayStatics.GetObjectClass` OtherActor) "/Game/FirstPerson/Blueprints/BP_FirstPersonCharacter.BP_FirstPersonCharacter_C")
    (for _index (range (+ (`GameplayStatics.GetNumLocalPlayerControllers`) 1))
      (bind _asbp_first_person_character (cast `/Game/FirstPerson/Blueprints/BP_FirstPersonCharacter` (`GameplayStatics.GetPlayerPawn` _index)))
      (`/Game/FirstPerson/Blueprints/BP_FirstPersonCharacter.DoublePointsActivated` _asbp_first_person_character))
    (`self.K2_DestroyActor`)))

(fn `UserConstructionScript`
  (`parent.UserConstructionScript`))