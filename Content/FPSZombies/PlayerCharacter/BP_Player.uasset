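; Player character for a first-person zombie shooter, handling Enhanced Input movement, sprinting, shooting, reloading and the HUD.
; Shooting repeats while held, gated by fire rate and ammo, using camera line traces to damage BP_Zombie and award money.
; Interact sphere-traces for purchasable doors that activate spawns, or quit the game if marked as escape.
; Death ragdolls the mesh, disables input and reloads ZombieMap; leftover aim and camera-arm logic never runs.
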(event `self.ReceiveBeginPlay`
  (`EnhancedInputSubsystemInterface.AddMappingContext` (pcsubsystem `EnhancedInputLocalPlayerSubsystem` (`GameplayStatics.GetPlayerController` 0)) "/Game/FPSZombies/Input/IMC_MovementAndLook.IMC_MovementAndLook" 0 (struct))
  (bind _returnvalue (`|CreateWidget` "/Game/FPSZombies/HUD/WB_UIHUD.WB_UIHUD_C"))
  (`UserWidget.AddToViewport` _returnvalue 0)
  (set `CharacterMovementComponent.MaxWalkSpeed` (`self.WalkSpeed`) (`self.CharacterMovement`)))

(event `EnhancedInput|/Game/FPSZombies/Input/IA_MoveForward`
  (params (ActionValue :type "Float (double-precision)") (ElapsedSeconds :type "Float (double-precision)") (TriggeredSeconds :type "Float (double-precision)") (InputAction :type "InputAction Object Reference" :default "/Game/FPSZombies/Input/IA_MoveForward.IA_MoveForward"))
  (bind (_returnvalue_roll _returnvalue_pitch _returnvalue_yaw) (`KismetMathLibrary.BreakRotator` (`self.GetControlRotation`)))
  (:`Triggered`
    (`self.AddMovementInput` (`KismetMathLibrary.GetForwardVector` (`KismetMathLibrary.MakeRotator` 0.0 0.0 _returnvalue_yaw)) ActionValue)))

(event `EnhancedInput|/Game/FPSZombies/Input/IA_LookUp`
  (params (ActionValue :type "Float (double-precision)") (ElapsedSeconds :type "Float (double-precision)") (TriggeredSeconds :type "Float (double-precision)") (InputAction :type "InputAction Object Reference" :default "/Game/FPSZombies/Input/IA_LookUp.IA_LookUp"))
  (:`Triggered`
    (`self.AddControllerPitchInput` ActionValue)))

(event `EnhancedInput|/Game/FPSZombies/Input/IA_LookRight`
  (params (ActionValue :type "Float (double-precision)") (ElapsedSeconds :type "Float (double-precision)") (TriggeredSeconds :type "Float (double-precision)") (InputAction :type "InputAction Object Reference" :default "/Game/FPSZombies/Input/IA_LookRight.IA_LookRight"))
  (:`Triggered`
    (`self.AddControllerYawInput` ActionValue)))

(event `EnhancedInput|/Game/FPSZombies/Input/IA_MoveRight`
  (params (ActionValue :type "Float (double-precision)") (ElapsedSeconds :type "Float (double-precision)") (TriggeredSeconds :type "Float (double-precision)") (InputAction :type "InputAction Object Reference" :default "/Game/FPSZombies/Input/IA_MoveRight.IA_MoveRight"))
  (bind (_returnvalue_roll _returnvalue_pitch _returnvalue_yaw) (`KismetMathLibrary.BreakRotator` (`self.GetControlRotation`)))
  (:`Triggered`
    (`self.AddMovementInput` (`KismetMathLibrary.GetRightVector` (`KismetMathLibrary.MakeRotator` 0.0 0.0 _returnvalue_yaw)) ActionValue)))

(event `EnhancedInput|/Game/FPSZombies/Input/IA_My_Jump`
  (params (ActionValue :type Boolean) (ElapsedSeconds :type "Float (double-precision)") (TriggeredSeconds :type "Float (double-precision)") (InputAction :type "InputAction Object Reference" :default "/Game/FPSZombies/Input/IA_My_Jump.IA_My_Jump"))
  (:`Triggered`
    (`self.Jump`)))

(event `EnhancedInput|/Game/FPSZombies/Input/IA_Sprint`
  (params (ActionValue :type Boolean) (ElapsedSeconds :type "Float (double-precision)") (TriggeredSeconds :type "Float (double-precision)") (InputAction :type "InputAction Object Reference" :default "/Game/FPSZombies/Input/IA_Sprint.IA_Sprint"))
  (bind _charactermovement (`self.CharacterMovement`))
  (:`Started`
    (set `self.AimingDownSights` false)
    (if (not (`self.AimingDownSights`))
      (set `CharacterMovementComponent.MaxWalkSpeed` (`self.SprintSpeed`) _charactermovement)))
  (:`Completed`
    (set `self.AimingDownSights` true)
    (set `CharacterMovementComponent.MaxWalkSpeed` (`self.WalkSpeed`) _charactermovement :!label _label)))

(event `Unsprint`
  (goto _label))

(event `EnhancedInput|/Game/FPSZombies/Input/IA_Aiming`
  (params (ActionValue :type Boolean) (ElapsedSeconds :type "Float (double-precision)") (TriggeredSeconds :type "Float (double-precision)") (InputAction :type "InputAction Object Reference" :default "/Game/FPSZombies/Input/IA_Aiming.IA_Aiming")))

(event `Shoot`
  (bind _muzzle (`self.Muzzle`))
  (bind _fps_camera (`self.FPS Camera`))
  (bind _returnvalue (`SceneComponent.K2_GetComponentLocation` _muzzle))
  (bind _returnvalue_2 (`SceneComponent.K2_GetComponentLocation` _fps_camera))
  (if (and (not (`self.Sprinting`)) (> (`self.CurrentAmmo`) 0)) :!label _label_2
    (set `self.CurrentAmmo` (- (`self.CurrentAmmo`) 1))
    (`GameplayStatics.SpawnEmitterAtLocation` "/Game/StarterContent/Particles/P_Explosion1.P_Explosion1" _returnvalue (`SceneComponent.K2_GetComponentRotation` _muzzle) (0.15 0.15 0.15))
    (`GameplayStatics.PlaySoundAtLocation` "/Game/Art/Sounds/ShotSoundCue.ShotSoundCue" _returnvalue (struct) 1.0 1.0 0.0 null null null null)
    (`PlayerController.ClientStartCameraShake` :`self` (`GameplayStatics.GetPlayerController` 0) :`Shake` "/Game/Blueprints/Misc/CS_Shoot.CS_Shoot_C")
    (bind (_outhit _returnvalue_3) (`KismetSystemLibrary.LineTraceSingle` _returnvalue_2 (+ _returnvalue_2 (* (`SceneComponent.GetForwardVector` _fps_camera) (`self.ShootingMultiplier`))) "TraceTypeQuery1"))
    (`|ExecutionSequence`
      (:`then_0`
        (set `self.CanShoot` false)
        (`KismetSystemLibrary.Delay` (`self.FireRate`))
        (set `self.CanShoot` true)
        (if (`self.LMBPressed`)
          (`self.Shoot`)))
      (:`then_1`
        (if _returnvalue_3
          (bind (_bblockinghit _binitialoverlap _time _distance _location _impactpoint _normal _impactnormal _physmat _hitactor) (`GameplayStatics.BreakHitResult` _outhit))
          (`GameplayStatics.SpawnEmitterAtLocation` "/Game/StarterContent/Particles/P_Explosion.P_Explosion" _location)
          (bind _asbp_zombie (cast `/Game/FPSZombies/ZombieBlueprints/BP_Zombie` _hitactor))
          (`/Game/FPSZombies/ZombieBlueprints/BP_Zombie.Deal Damage` _asbp_zombie (`self.Damage`))
          (set `self.Money` (+ (`self.Money`) (`/Game/FPSZombies/ZombieBlueprints/BP_Zombie.Hit Score` _asbp_zombie))))))))

(event `EnhancedInput|/Game/FPSZombies/Input/IA_Shoot`
  (params (ActionValue :type Boolean) (ElapsedSeconds :type "Float (double-precision)") (TriggeredSeconds :type "Float (double-precision)") (InputAction :type "InputAction Object Reference" :default "/Game/FPSZombies/Input/IA_Shoot.IA_Shoot"))
  (:`Started`
    (set `self.LMBPressed` true)
    (if (`self.CanShoot`)
      (goto _label_2)))
  (:`Completed`
    (set `self.LMBPressed` false)))

(event `EnhancedInput|/Game/FPSZombies/Input/IA_Reload`
  (params (ActionValue :type Boolean) (ElapsedSeconds :type "Float (double-precision)") (TriggeredSeconds :type "Float (double-precision)") (InputAction :type "InputAction Object Reference" :default "/Game/FPSZombies/Input/IA_Reload.IA_Reload"))
  (:`Started`
    (if (`AnimInstance.Montage_IsPlaying` (`SkeletalMeshComponent.GetAnimInstance` (`self.Mesh`)) "/Game/Art/Mannequin/Animations/AnimStarterPack/Reload_Rifle_Hip_Montage.Reload_Rifle_Hip_Montage")
      _
      (elif (< (`self.CurrentAmmo`) (`self.MaxAmmo`))
        (set `self.CanShoot` false)
        (bind _returnvalue (`AnimInstance.Montage_Play` (`SkeletalMeshComponent.GetAnimInstance` (`self.Mesh`)) "/Game/Art/Mannequin/Animations/AnimStarterPack/Reload_Rifle_Hip_Montage.Reload_Rifle_Hip_Montage" 1.0 "MontageLength" 0.0 true))
        (`|ExecutionSequence`
          (:`then_0`
            (`KismetSystemLibrary.Delay` _returnvalue)
            (set `self.CurrentAmmo` (`self.MaxAmmo`))
            (set `self.CanShoot` true))
          (:`then_1`
            (`KismetSystemLibrary.Delay` 0.4)
            (`GameplayStatics.PlaySoundAtLocation` "/Game/Art/Sounds/AssaultRifle_Reload.AssaultRifle_Reload" (`self.K2_GetActorLocation`) (struct) 1.0 1.0 0.0 null null null null)))))))

(event `Deal Damage`
  (params (Damage :type "Float (double-precision)"))
  (bind _output_get (set `self.Health` (- (`self.Health`) Damage)))
  (if (<= _output_get 0.0)
    (set `self.LMBPressed` false)
    (set `self.CanShoot` false)
    (`PrimitiveComponent.SetSimulatePhysics` (`self.Mesh`) true)
    (`self.DisableInput` (`GameplayStatics.GetPlayerController` 0))
    (`self.Unsprint`)
    (`KismetSystemLibrary.Delay` 2.0)
    (`GameplayStatics.OpenLevelBySoftObjectPtr` "/Game/Levels/ZombieMap.ZombieMap")))

(event `EnhancedInput|/Game/FPSZombies/Input/IA_Interact`
  (params (ActionValue :type Boolean) (ElapsedSeconds :type "Float (double-precision)") (TriggeredSeconds :type "Float (double-precision)") (InputAction :type "InputAction Object Reference" :default "/Game/FPSZombies/Input/IA_Interact.IA_Interact"))
  (bind _fps_camera (`self.FPS Camera`))
  (bind _returnvalue (`SceneComponent.K2_GetComponentLocation` _fps_camera))
  (:`Started`
    (bind (_outhit _returnvalue_2) (`KismetSystemLibrary.SphereTraceSingle` :`Start` _returnvalue :`End` (+ _returnvalue (* (`KismetMathLibrary.GetForwardVector` (`SceneComponent.K2_GetComponentRotation` _fps_camera)) 200)) :`Radius` 100.0 :`TraceChannel` "TraceTypeQuery1" :`DrawTime` 3.0))
    (if _returnvalue_2
      (bind _asbp_double_sliding_door (cast `/Game/FPSZombies/DoorBlueprints/BP_DoubleSlidingDoor` (`.HitActor` (`GameplayStatics.BreakHitResult` _outhit))))
      (bind _price (`/Game/FPSZombies/DoorBlueprints/BP_DoubleSlidingDoor.Price` _asbp_double_sliding_door))
      (if (<= _price (`self.Money`))
        (set `self.Money` (- (`self.Money`) _price))
        (if (`/Game/FPSZombies/DoorBlueprints/BP_DoubleSlidingDoor.IsEscape` _asbp_double_sliding_door)
          (`KismetSystemLibrary.QuitGame` null "Quit")
          (else
            (`/Game/FPSZombies/DoorBlueprints/BP_DoubleSlidingDoor.ActivateSpawns` _asbp_double_sliding_door)
            (`self.K2_DestroyActor` _asbp_double_sliding_door)))))))

(fn `Increment Kill Count`
  (set `self.KillCounter` (+ (`self.KillCounter`) 1)))

(fn `UserConstructionScript`)