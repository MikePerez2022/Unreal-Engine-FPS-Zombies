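; BP_DoubleSlidingDoor is a door in a zombie FPS that shows an interaction prompt with a price and an escape flag.
; On BeginPlay it creates a WB_Interact widget and passes it Price and IsEscape.
; The MsgBox overlap volume adds the prompt to the viewport when the player character enters and removes it on exit.
; ActivateSpawns switches on the linked Spawners, while purchase and sliding logic are absent here.
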(event `self.ReceiveBeginPlay`
  (bind _returnvalue (`|GenericCreateObject` "/Game/FPSZombies/HUD/WB_Interact.WB_Interact_C"))
  (bind _output_get (set `self.InteractPromp` _returnvalue))
  (`/Game/FPSZombies/HUD/WB_Interact.Set Price` _output_get (`self.Price`))
  (`/Game/FPSZombies/HUD/WB_Interact.Set Is Escape` _output_get (`self.IsEscape`)))

(event `self.MsgBox.OnComponentBeginOverlap`
  (params (OverlappedComponent :type "PrimitiveComponent Object Reference") (OtherActor :type "Actor Object Reference") (OtherComp :type "PrimitiveComponent Object Reference") (OtherBodyIndex :type Integer) (bFromSweep :type Boolean) (SweepResult :type "HitResult Structure (by ref)"))
  (if (== OtherActor (`GameplayStatics.GetPlayerCharacter` 0))
    (`UserWidget.AddToViewport` (`self.InteractPromp`) 0)))

(event `self.MsgBox.OnComponentEndOverlap`
  (params (OverlappedComponent :type "PrimitiveComponent Object Reference") (OtherActor :type "Actor Object Reference") (OtherComp :type "PrimitiveComponent Object Reference") (OtherBodyIndex :type Integer))
  (if (== (`GameplayStatics.GetPlayerCharacter` 0) OtherActor)
    (`Widget.RemoveFromParent` (`self.InteractPromp`))))

(fn `ActivateSpawns`
  (for _array_element (`self.Spawners`)
    (set `/Game/FPSZombies/SpawnerBlueprints/BP_Zombie_Spawner.Is Active` true _array_element)))

(fn `UserConstructionScript`)